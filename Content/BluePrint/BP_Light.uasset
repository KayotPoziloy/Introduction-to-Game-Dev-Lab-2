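; BP_Light is a spotlight that blinks a set number of times when play begins.
; The construction script sets its initial visibility from IsEnable.
; BeginPlay runs a DoN and Delay loop that toggles visibility every Duration.
; The toggle total is Count times two minus one, an odd number for positive counts, so the light ends opposite to its starting state.
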(event `self.ReceiveBeginPlay`
  (bind _returnvalue (`self.*2-1` (`self.count`)))
  (`/Engine/EditorBlueprintResources/StandardMacros.Do N` _returnvalue :!label _label
    (:`Exit`
      (`KismetSystemLibrary.Delay` (`self.duration`))
      (`SceneComponent.ToggleVisibility` (`self.SpotLight`) false)
      (goto _label))))

(fn `*2-1`
  (params (int :type Integer))
  (returns (ReturnValue :type Integer))
  (return (- (* int 2) 1)))

(fn `UserConstructionScript`
  (`SceneComponent.SetVisibility` (`self.SpotLight`) (`self.is_enable`) false))